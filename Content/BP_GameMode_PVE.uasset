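; BP_GameMode_PVE is a PVE game mode Blueprint whose only logic is a deprecated debug goal-post spawner, noted as moved into BP_GoalPost itself.
; CreateGoalPost spawns a BP_GoalPost at a random point in a box around the origin, prints the position, destroys it after a short delay, then calls itself again.
; Nothing starts that loop, as BeginPlay and the construction script are empty and the other call is disconnected.
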(event `self.ReceiveBeginPlay`)

(event `Create goal post`
  ;[0.15 0.08075 0 0.5] debug - spawn a point in the court for player to go after ->deprecated! This logic is put in BP_goalPost itself. drag one in the scene and it should work.
  (set `self.Goal Position` (`KismetMathLibrary.RandomPointInBoundingBox` (0.0 0.0 0.0) (200.0 200.0 10.0)))
  (`KismetSystemLibrary.PrintString` (`KismetStringLibrary.Concat_StrStr` "Goal Position: " (`KismetStringLibrary.Conv_VectorToString` (`self.Goal Position`))))
  (bind _returnvalue (`|SpawnActorFromClass` "/Game/BP_GoalPost.BP_GoalPost_C" (`KismetMathLibrary.Conv_VectorToTransform` (`self.Goal Position`)) "Undefined" "MultiplyWithRoot" null (0.0 0.0 0.0) null))
  (`KismetSystemLibrary.Delay` 3.0)
  (`self.K2_DestroyActor` _returnvalue)
  (`self.Create goal post`))

(fn `UserConstructionScript`)