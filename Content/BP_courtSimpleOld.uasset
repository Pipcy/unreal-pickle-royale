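; BP_courtSimpleOld is a court Blueprint with left and right service-area collision components, apparently an older version of a simple court.
; Both service-area begin-overlap events are empty, so the asset currently runs no logic.
; Disconnected graph fragments check for a "ball" tag, print debug text, then call CheckAndUpdate(false) on the BP_GamePractice game mode.
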(event `self.AServiceAreaLeft.OnComponentBeginOverlap`
  (params (OverlappedComponent :type "PrimitiveComponent Object Reference") (OtherActor :type "Actor Object Reference") (OtherComp :type "PrimitiveComponent Object Reference") (OtherBodyIndex :type Integer) (bFromSweep :type Boolean) (SweepResult :type "HitResult Structure (by ref)"))
  ;[0.15 0.08496 0 0.5] collision triggered upates
)

(event `self.AServiceAreaRight.OnComponentBeginOverlap`
  (params (OverlappedComponent :type "PrimitiveComponent Object Reference") (OtherActor :type "Actor Object Reference") (OtherComp :type "PrimitiveComponent Object Reference") (OtherBodyIndex :type Integer) (bFromSweep :type Boolean) (SweepResult :type "HitResult Structure (by ref)"))
  ;[0.15 0.08496 0 0.5] collision triggered upates
)

(fn `UserConstructionScript`)