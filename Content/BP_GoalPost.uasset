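; BP_GoalPost is a debug actor meant to give the player a target point inside the court.
; BeginPlay calls UpdateGoalPost, but that event is disconnected because the court changed, so it currently does nothing.
; The orphaned chain picks a random point in BP_courtSimple's BServiceArea box, moves the actor there, prints it, and repeats every eight seconds.
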(event `self.ReceiveBeginPlay`
  (`self.UpdateGoalPost`))

(event `UpdateGoalPost`
  ;[0.15 0.1265 0.03049 0.5] debug - spawn a point in the court for player to go after (disconnect because the court changed)
)

(fn `UserConstructionScript`)