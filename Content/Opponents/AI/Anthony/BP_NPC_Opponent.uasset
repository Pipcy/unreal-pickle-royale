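; BP_NPC_Opponent is an NPC opponent with a paddle, set up for a ball game with serves.
; Tick caches the paddle mesh's world location, while BeginPlay and OpponentServe are empty.
; Disconnected serve logic clears existing ball projectiles, solves an arced launch velocity toward a target bounce point, and spawns a new BP_Ball_Projectile heading to side A.
; That logic never runs, so the opponent does not currently serve.
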(event `self.ReceiveTick`
  (params (DeltaSeconds :type "Float (single-precision)"))
  (set `self.Paddle Mesh Location Ref` (`SceneComponent.K2_GetComponentLocation` (`self.paddle Mesh`))))

(event `self.ReceiveBeginPlay`)

(event `Opponent Serve`
  ;[0.15 0.1094 0.01284 0.5] opponent serve
)

(fn `UserConstructionScript`)