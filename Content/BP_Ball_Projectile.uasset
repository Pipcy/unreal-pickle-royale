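; Ball projectile for a net-and-court sport that detects bounces and outs and awards points through BP_GamemodeFirstTo3.
; Overlaps with tagged court areas, debounced by time, record the last two bounce zones, which are checked against the heading tag to catch short shots.
; Floor-plane hits outside the BP_CourtAreaInAir zone score by heading and bounce count.
; SetBallHeadingState, meant for swings, clears bounce history when direction changes.
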(event `self.ReceiveBeginPlay`
  (bind _projectilemovement (`self.ProjectileMovement`))
  ; set this on spawn
  (set `MovementComponent.Velocity` (`self.Velocity`) _projectilemovement)
  (set `ProjectileMovementComponent.ProjectileGravityScale` (`self.GravityScale`) _projectilemovement)
  ; set up the air zone check BP
  (bind _returnvalue (`GameplayStatics.GetActorOfClass` "/Game/BP_CourtAreaInAir.BP_CourtAreaInAir_C"))
  (set `self.Ball air zone check BP` _returnvalue)
  ;[0.15 0.03507 0.04854 0.5] gamemode TOFIX
  (bind _asbp_gamemode_first_to_3 (cast `/Game/Levels/BP_GamemodeFirstTo3` (`GameplayStatics.GetGameMode`)))
  (set `self.Gamemode ref` _asbp_gamemode_first_to_3))

(event `self.ReceiveTick`
  (params (DeltaSeconds :type "Float (single-precision)"))
  ; update world location live
  (set `self.Current World Location` (`SceneComponent.K2_GetComponentLocation` (`self.Sphere`))))

(event `On Ball Heading State Changed`
  ; reset data once heading direction switched
  (set `self.Ball Bounce Count` 0)
  (set `self.Most Recent Bounce Area` "NewEnumerator7")
  (set `self.Second Most Recent Bounce Area` "NewEnumerator7"))

(event `self.Sphere.OnComponentHit`
  (params (HitComponent :type "PrimitiveComponent Object Reference") (OtherActor :type "Actor Object Reference") (OtherComp :type "PrimitiveComponent Object Reference") (NormalImpulse :type "Vector Structure") (Hit :type "HitResult Structure (by ref)"))
  ; for Hit event (an "Out")
  (if (`self.ball is Active?`)
    (if (and (`ActorComponent.ComponentHasTag` OtherComp "floor plane") (not (`/Game/BP_CourtAreaInAir.Ball in Court Air Zone?` (`self.Ball air zone check BP`))))
      (`KismetSystemLibrary.PrintString` "OUT" true true (struct :`R` 1.0 :`G` 0.268976 :`B` 0.966077 :`A` 1.0))
      (if (< (`self.Ball Bounce Count`) 1)
        (`|SwitchGameplayTag` (`self.Ball Heading State`) ; ball is out
          (:`Ball.HeadingTo.Aside`
            (`/Game/Levels/BP_GamemodeFirstTo3.Increment Player Score` (`self.Gamemode ref`) :!label _label))
          (:`Ball.HeadingTo.Bside`
            (`/Game/Levels/BP_GamemodeFirstTo3.Increment Opponent Score` (`self.Gamemode ref`) :!label _label_2)))
        (else
          (`|SwitchGameplayTag` (`self.Ball Heading State`) ; this happens with the first bounce is in and second bounce is out (swing miss)
            (:`Ball.HeadingTo.Aside`
              (goto _label_2))
            (:`Ball.HeadingTo.Bside`
              (goto _label)))))
      (set `self.Ball Heading State` (struct :`TagName` "Ball.HeadingTo.Nowhere"))
      (set `self.ball is Active?` false))))

(event `self.Sphere.OnComponentBeginOverlap`
  (params (OverlappedComponent :type "PrimitiveComponent Object Reference") (OtherActor :type "Actor Object Reference") (OtherComp :type "PrimitiveComponent Object Reference") (OtherBodyIndex :type Integer) (bFromSweep :type Boolean) (SweepResult :type "HitResult Structure (by ref)"))
  ; for overlap event (determine the area of the court the ball land in)
  (if (`self.ball is Active?`)
    (bind _trigger_is_court_area_bounce (`self.Check if trigger is a valid court area bounce` OtherComp)) ; beyond this point it should only be bounce in court areas
    (if _trigger_is_court_area_bounce
      (`self.Register Bounce info` OtherComp)
      (`self.On Bounce Info Updated`))))

(event `On Bounce Info Updated`
  ; check the rules based on bounce updates
  (`|SwitchGameplayTag` (`self.Ball Heading State`)
    (:`Ball.HeadingTo.Aside`
      (switch `/Game/Opponents/AI/Anthony/Enums/Enum_CourtAreas` (`self.Most Recent Bounce Area`)
        (:`NewEnumerator0`
          (switch `/Game/Opponents/AI/Anthony/Enums/Enum_CourtAreas` (`self.Second Most Recent Bounce Area`)
            (:`NewEnumerator0`
              (`KismetSystemLibrary.PrintString` "player didn't make the ball pass the net (A side short)" true true (struct :`R` 1.0 :`B` 0.085713 :`A` 1.0) :!label _label_3)
              (`/Game/Levels/BP_GamemodeFirstTo3.Increment Opponent Score` (`self.Gamemode ref`))
              (set `self.ball is Active?` false)
              (set `self.Ball Heading State` (struct :`TagName` "Ball.HeadingTo.Nowhere")))
            (:`NewEnumerator7`
              (`KismetSystemLibrary.PrintString` "good" true true (struct :`R` 0.036935 :`G` 1.0 :`A` 1.0)))))
        (:`NewEnumerator4`
          (`KismetSystemLibrary.PrintString` "Opponent didn't make the ball pass the net (B side short)" true true (struct :`R` 1.0 :`G` 0.114338 :`B` 0.134234 :`A` 1.0) :!label _label_4)
          (`/Game/Levels/BP_GamemodeFirstTo3.Increment Player Score` (`self.Gamemode ref`))
          (set `self.ball is Active?` false)
          (set `self.Ball Heading State` (struct :`TagName` "Ball.HeadingTo.Nowhere")))))
    (:`Ball.HeadingTo.Bside`
      (switch `/Game/Opponents/AI/Anthony/Enums/Enum_CourtAreas` (`self.Most Recent Bounce Area`) ; opponent hit but ball bounce on B again
        (:`NewEnumerator0`
          (goto _label_3))
        (:`NewEnumerator4`
          (switch `/Game/Opponents/AI/Anthony/Enums/Enum_CourtAreas` (`self.Second Most Recent Bounce Area`)
            (:`NewEnumerator4`
              (goto _label_4))
            (:`NewEnumerator7`
              (`KismetSystemLibrary.PrintString` "good" true true (struct :`R` 0.081203 :`G` 1.0 :`A` 1.0)))))))))

(fn `Check if trigger is a valid court area bounce`
  (params (`Collision Component` :type "ActorComponent Object Reference"))
  (returns (`Trigger is court area Bounce` :type Boolean))
  ; If ball collides with court floor
  (if (`ActorComponent.ComponentHasTag` `Collision Component` "court area")
    ; check trigger time delta to avoid back-to-back trigger
    (if (> (- (`KismetSystemLibrary.GetGameTimeInSeconds`) (`self.Last Bounce Trigger Time`)) 0.01)
      (return true))
    (else
      (return false))))

(fn `Register Bounce info`
  (params (InputPin :type "PrimitiveComponent Object Reference"))
  ; register bounce
  ;; categorize this bounce to either A or B zone
  (if (`ActorComponent.ComponentHasTag` InputPin "Zone_A")
    (set `self.Bounce Location` "NewEnumerator0") ; should only be the FULL area, not using individual
    (else
      (bind _output_get (set `self.Bounce Location` "NewEnumerator4"))))
  (`KismetSystemLibrary.PrintString` (`|GetEnumeratorNameAsString` _output_get) false true (struct :`R` 1.0 :`G` 0.885502 :`A` 1.0))
  (`/Engine/EditorBlueprintResources/StandardMacros.IncrementInt` (`self.Ball Bounce Count`)
    (:`  `
      (`KismetSystemLibrary.PrintString` (`KismetSystemLibrary.GetDisplayName` InputPin) false true (struct :`R` 1.0 :`G` 0.851208 :`A` 1.0))
      (set `self.Last Bounce Trigger Time` (`KismetSystemLibrary.GetGameTimeInSeconds`))
      (bind _output_get_2 (set `self.Second Most Recent Bounce Area` (`self.Most Recent Bounce Area`)))
      (bind _output_get_3 (set `self.Most Recent Bounce Area` (`self.Bounce Location`)))
      (`KismetSystemLibrary.PrintString` (`KismetStringLibrary.Concat_StrStr` (`|GetEnumeratorNameAsString` _output_get_2) (`|GetEnumeratorNameAsString` _output_get_3)) true true (struct :`R` 1.0 :`G` 0.762732 :`A` 1.0)))))

(fn `Set Ball Heading State`
  (params (`New Ball Heading State` :type "GameplayTag Structure"))
  (if (!= `New Ball Heading State` (`self.Ball Heading State`))
    (set `self.Ball Heading State` `New Ball Heading State`)
    (`self.On Ball Heading State Changed`)))

(fn `UserConstructionScript`)