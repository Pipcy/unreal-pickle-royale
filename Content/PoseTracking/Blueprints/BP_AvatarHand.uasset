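; BP_AvatarHand moves a test cube to follow the first Nuitrack user's right hand, as a hand-tracking prototype.
; On BeginPlay it requires a BP_NuitrackManager in the level, then starts a looping timer at about 60 Hz.
; Each update places the cube at the scaled joint position offset by TrackingOrigin, if confidence meets the threshold.
; Left-handed tracking only prints a message, and the user list is indexed without an empty check.
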(event `self.ReceiveBeginPlay`
  ;[0.4167 0.4167 0.4167] Init
  (bind _outactors (`GameplayStatics.GetAllActorsOfClass` "/NuitrackPlugin/Blueprints/BP_NuitrackManager.BP_NuitrackManager_C"))
  (if (> (`KismetArrayLibrary.Array_Length` _outactors) 0)
    (set `self.isRightHanded` true)
    (set `self.jointConfidenceThreshhold` 0.5)
    ;; update 60z = 0.016 s
    (`KismetSystemLibrary.K2_SetTimerDelegate` (delegate `UpdateHand`) 0.016 true true)
    (else
      (`KismetSystemLibrary.PrintString` "Nuitrack Manager was not found!  \nPlace BP_NuitrackManager on the level" true true (struct :`R` 1.0 :`B` 0.066667 :`A` 1.0) 10.0))))

(event `UpdateHand`
  ; define UpdateHand event behavior
  (bind _returnvalue (`NuitrackUtils.GetUsers`))
  (`KismetSystemLibrary.PrintString` (`KismetStringLibrary.Concat_StrStr` "GetUsers length: " (`KismetStringLibrary.Conv_IntToString` (`KismetArrayLibrary.Array_Length` _returnvalue))) true true (struct :`G` 0.66 :`B` 1.0 :`A` 1.0) 0.1)
  (if (`self.isRightHanded`)
    (bind (_transform3d _projectionpos _confidence) (`NuitrackUtils.GetJoint` (`.skeleton` (break `NuitrackUser` (`|GetArrayItem` _returnvalue))) "JOINT_RIGHT_HAND"))
    (`KismetSystemLibrary.PrintString` (`KismetStringLibrary.Concat_StrStr` "Get Joint Confidence: " (`KismetStringLibrary.Conv_DoubleToString` _confidence)) false true (struct :`G` 0.66 :`B` 1.0 :`A` 1.0) 0.02)
    ;; confidence check
    (if (>= _confidence (`self.jointConfidenceThreshhold`))
      ;; actually update position
      (`SceneComponent.K2_SetWorldLocation` (`self.TestCube`) (+ (* (2.0 2.0 2.0) (.location _transform3d)) (`SceneComponent.K2_GetComponentLocation` (`self.TrackingOrigin`))) false false)
      (else
        (`KismetSystemLibrary.PrintString` "uh oh, not confident enough" false true (struct :`G` 0.66 :`B` 1.0 :`A` 1.0) 0.02)))
    (else
      (`KismetSystemLibrary.PrintString` "uh oh, you're left handed"))))

(fn `UserConstructionScript`)