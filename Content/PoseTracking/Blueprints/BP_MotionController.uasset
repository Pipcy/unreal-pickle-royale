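; BP_MotionController is an actor that mirrors a player's physical motion, taking position from Nuitrack/Kinect right-hand tracking and rotation from CSV Euler angles received over UDP.
; A 60 Hz timer remaps and smooths hand position, then checks recent height history for swings, which are only printed.
; Incoming angles are axis-swapped, clamped relative to a calibrated yaw with pitch zeroed, then exponentially smoothed on Tick.
; BeginPlay also creates a calibration button widget.
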(event `self.ReceiveBeginPlay`
  (bind _returnvalue (`GameplayStatics.GetPlayerController` 0))
  (`KismetSystemLibrary.Delay` 0.2)
  (set `self.CalibratedZero` (struct :`Yaw` 50.0))
  (set `self.AdjustedAlpha` 0.5)
  (set `self.ClampConfig` (make `/Game/PoseTracking/Blueprints/MotionClampLimits` -20.0 20.0 130.0 -130.0 -80.0 80.0))
  (set `self.AdjustedEulerX` 0.0)
  (set `self.PrevLocation` (0.0 0.0 0.0))
  (set `self.PrevRotator` (struct))
  (bind _setupcomplete (`self.SetupDevices`))
  (if _setupcomplete
    (`KismetSystemLibrary.K2_SetTimerDelegate` (delegate `UpdatePosition`) 0.016 true) ; 60 Hz = 0.016 s
  )
  ; create calibration widget (button)
  (bind _returnvalue_2 (`|CreateWidget` "/Game/PoseTracking/Blueprints/WB_CalibrateButton.WB_CalibrateButton_C" _returnvalue self))
  (`UserWidget.AddToViewport` _returnvalue_2 0)
  (set `PlayerController.bShowMouseCursor` true _returnvalue)
  (`WidgetBlueprintLibrary.SetInputMode_GameAndUIEx` _returnvalue _returnvalue_2)
  (`KismetSystemLibrary.PrintString` "BP_MC created widget" true false))

(event `self.WirelessUDP.OnReceiveSocketOpened`
  (params (Port :type Integer))
  (`KismetSystemLibrary.PrintString` (`KismetStringLibrary.Concat_StrStr` "Receive socket listening on port " (`KismetStringLibrary.Conv_IntToString` Port)) true false (struct :`R` 1.0 :`G` 1.0 :`B` 1.0 :`A` 1.0) 5.0))

(event `self.ReceiveTick`
  (params (DeltaSeconds :type "Float (single-precision)"))
  ; every tick, compute alpha = 1 - exp(-speed * deltaSeconds)
  (bind _output_get (set `self.AdjustedAlpha` (- 1.0 (`KismetMathLibrary.Exp` (* (* 16.0 -1.0) DeltaSeconds)))))
  (bind _returnvalue (`KismetMathLibrary.RLerp` (`self.PrevRotator`) (stale `self.WirelessUDP.OnReceivedBytes` _clampedrotator) _output_get true))
  ; lerp from previous rotation and set actor rotation
  (`self.K2_SetActorRotation` _returnvalue)
  (set `self.PrevRotator` _returnvalue))

(event `self.WirelessUDP.OnReceivedBytes`
  (params (Bytes :type "Array of Byte (by ref)") (IPAddress :type String) (Port :type "Integer (by ref)"))
  (`KismetSystemLibrary.PrintString` (`KismetStringLibrary.Concat_StrStr` "Receiving: " (`CUBlueprintLibrary.Conv_BytesToString` Bytes)) true false (struct :`R` 0.677083 :`G` 0.677083 :`B` 0.677083 :`A` 1.0) 0.1)
  (bind (_euler_x _euler_y _euler_z) (`self.ParseCSV` Bytes))
  (bind (_eulerx _eulery _eulerz) (`self.SwapAxes` _euler_x _euler_y _euler_z))
  (set `self.CurrentZ` _eulerz)
  (bind _clampedrotator (`self.GetClampedRotator` _eulerx _eulery _eulerz)) ; X is roll, Y is pitch, Z is yaw
)

(event `UpdatePosition`
  (bind _returnvalue (`NuitrackUtils.GetUsers`))
  (if (> (`KismetArrayLibrary.Array_Length` _returnvalue) 0)
    (bind (_transform3d _projectionpos _confidence) (`NuitrackUtils.GetJoint` (`.skeleton` (break `NuitrackUser` (`|GetArrayItem` _returnvalue))) "JOINT_RIGHT_HAND"))
    (if (> _confidence 0.3)
      (bind _returnvalue_2 (`KismetMathLibrary.MakeVector` (* (.y (* (+ (.location _transform3d) (`KismetMathLibrary.MakeVector` 0.0 0.0 70.0)) (1.0 1.0 1.0))) -1.0) (.x (* (+ (.location _transform3d) (`KismetMathLibrary.MakeVector` 0.0 0.0 70.0)) (1.0 1.0 1.0))) (.z (* (+ (.location _transform3d) (`KismetMathLibrary.MakeVector` 0.0 0.0 70.0)) (1.0 1.0 1.0)))))
      (`self.K2_SetActorLocation` (`KismetMathLibrary.VLerp` (`self.PrevLocation`) _returnvalue_2 0.5))
      (set `self.PrevLocation` _returnvalue_2)
      (bind _z (.z _returnvalue_2))
      ; log position values
      (`KismetSystemLibrary.PrintString` (`KismetStringLibrary.Concat_StrStr` (`KismetStringLibrary.Conv_DoubleToString` (.x _returnvalue_2)) (`KismetStringLibrary.Concat_StrStr` "," (`KismetStringLibrary.Concat_StrStr` (`KismetStringLibrary.Conv_DoubleToString` (.y _returnvalue_2)) (`KismetStringLibrary.Concat_StrStr` "," (`KismetStringLibrary.Conv_DoubleToString` _z))))) false)
      (bind _swingisdetected (`self.DetectSwing` _z))
      (if _swingisdetected
        (`KismetSystemLibrary.PrintString` (`KismetStringLibrary.Conv_BoolToString` _swingisdetected) true true (struct :`R` 1.0 :`B` 0.651564 :`A` 1.0) 0.5))
      (else
        (`KismetSystemLibrary.PrintString` "low confidence :(" true false (struct :`R` 0.322917 :`G` 0.028735 :`A` 1.0) 0.016)))
    (else
      (`KismetSystemLibrary.PrintString` "nobody detected :(" false true (struct :`R` 0.270833 :`B` 0.007835 :`A` 1.0) 0.016))))

(fn `DetectSwing`
  (params (CurrentZPosition :type "Float (double-precision)"))
  (returns (SwingIsDetected :type Boolean))
  (locals (ZDrop :type "Float (double-precision)"))
  (set `self.ZPos-0` CurrentZPosition)
  (set `self.ZVelocity` (- (`self.ZPos-0`) (`self.Z-1`)))
  (bind _max (`self.MaxOfSix` (`self.ZPos-0`) (`self.Z-1`) (`self.Z-2`) (`self.Z-3`) (`self.Z-4`) (`self.Z-5`)))
  (bind _output_get (set `self.ZRecentMax` _max))
  (set `local.ZDrop` (- _output_get (`self.ZPos-0`)))
  (set `self.Z-5` (`self.Z-4`))
  (set `self.Z-4` (`self.Z-3`))
  (set `self.Z-3` (`self.Z-2`))
  (set `self.Z-2` (`self.Z-1`))
  (set `self.Z-1` (`self.ZPos-0`))
  (set `self.ZPos-1` (`self.ZPos-0`))
  (return (or (> (`self.ZVelocity`) 0.1) (< (`local.ZDrop`) -10.0))))

(fn `GetClampedRotator`
  (params (EulerX :type "Float (double-precision)") (EulerY :type "Float (double-precision)") (EulerZ :type "Float (double-precision)"))
  (returns (ClampedRotator :type "Rotator Structure"))
  (locals (_x :type "Float (double-precision)") (_y :type "Float (double-precision)") (_z :type "Float (double-precision)") (_RelativeZ :type "Float (double-precision)"))
  (bind __y (`local._y`))
  (bind (_eulerxmin _eulerxmax) (break `/Game/PoseTracking/Blueprints/MotionClampLimits` (`self.ClampConfig`)))
  (bind (_eulerxmin_2 _eulerxmax_2 _eulerymin _eulerymax _eulerzmin) (break `/Game/PoseTracking/Blueprints/MotionClampLimits` (`self.ClampConfig`)))
  (bind (_eulerxmin_3 _eulerxmax_3 _eulerymin_2 _eulerymax_2 _eulerzmin_2 _eulerzmax) (break `/Game/PoseTracking/Blueprints/MotionClampLimits` (`self.ClampConfig`)))
  ; store angles locally
  (set `local._x` EulerX)
  (set `local._y` EulerY)
  (set `local._z` EulerZ)
  ;[0.5 0 0 0.5] check X axis rotation
  (if (< (`local._x`) _eulerxmin)
    (set `local._x` _eulerxmin)
    (elif (> (`local._x`) _eulerxmax)
      (set `local._x` _eulerxmax)))
  ;[0 0.25 0 0.5] check Y axis rotation
  (if (or (< __y -140.0) (> __y 140.0))
    _
    (elif (>= (`local._y`) 0.0)
      (set `local._y` 140.0)
      (else
        (set `local._y` -140.0))))
  ;[0 0 0.5 0.5] check Z axis rotation
  (bind _output_get (set `local._RelativeZ` (- (`local._z`) (.yaw (`self.CalibratedZero`)))))
  (`KismetSystemLibrary.PrintString` (`KismetStringLibrary.Concat_StrStr` "relative Z: " (`KismetStringLibrary.Conv_DoubleToString` _output_get)) false false (struct :`G` 0.66 :`B` 1.0 :`A` 1.0) 0.3)
  ;;[0 0 0.5 0.5] unwrap Z so that relative Z has no discontinuity
  (if (not (< (`KismetMathLibrary.Abs` (- (`local._z`) (.yaw (`self.PrevRotator`)))) 180.0))
    (set `local._RelativeZ` (- (`local._z`) (.yaw (`self.CalibratedZero`)))) ; account for calibrated zero orientation
  )
  ; detect the snappage
  (if (> (`KismetMathLibrary.Abs` (- (`local._RelativeZ`) (`self.PrevRelativeZ`))) 150.0)
    (set `local._RelativeZ` (- (`local._RelativeZ`) 360.0)))
  (`KismetSystemLibrary.PrintString` (`KismetStringLibrary.Concat_StrStr` "Relative Z: " (`KismetStringLibrary.Conv_DoubleToString` (`local._RelativeZ`))) false false)
  (if (> (`local._RelativeZ`) _eulerzmax)
    (set `local._RelativeZ` _eulerzmax)
    (elif (< (`local._RelativeZ`) _eulerzmin)
      (set `local._RelativeZ` _eulerzmin)))
  (set `self.PrevRelativeZ` (`local._RelativeZ`))
  ; if we detect a Z snap, default to the previous Z rotation. otherwise update with the new one
  (return (`KismetMathLibrary.MakeRotator` (`local._x`) 0.0 (`local._RelativeZ`))))

(fn `MaxOfSix`
  (params (Var1 :type "Float (double-precision)") (Var2 :type "Float (double-precision)") (Var3 :type "Float (double-precision)") (Var4 :type "Float (double-precision)") (Var5 :type "Float (double-precision)") (Var6 :type "Float (double-precision)"))
  (returns (Max :type "Float (double-precision)"))
  (return (`KismetMathLibrary.FMax` (`KismetMathLibrary.FMax` (`KismetMathLibrary.FMax` Var1 Var2) (`KismetMathLibrary.FMax` Var3 Var4)) (`KismetMathLibrary.FMax` Var5 Var6))))

(fn `ParseCSV`
  (params (`CSV Bytes` :type "Array of Byte"))
  (returns (euler_x :type "Float (double-precision)") (euler_y :type "Float (double-precision)") (euler_z :type "Float (double-precision)") (a :type "Float (double-precision)") (b :type "Float (double-precision)") (c :type "Float (double-precision)") (d :type "Float (double-precision)"))
  (bind _returnvalue (`KismetStringLibrary.ParseIntoArray` (`CUBlueprintLibrary.Conv_BytesToString` `CSV Bytes`) ","))
  (return (`KismetStringLibrary.Conv_StringToDouble` (`|GetArrayItem` _returnvalue)) (`KismetStringLibrary.Conv_StringToDouble` (`|GetArrayItem` _returnvalue 1)) (`KismetStringLibrary.Conv_StringToDouble` (`|GetArrayItem` _returnvalue 2)) (`KismetStringLibrary.Conv_StringToDouble` (`|GetArrayItem` _returnvalue 3)) (`KismetStringLibrary.Conv_StringToDouble` (`|GetArrayItem` _returnvalue 4)) (`KismetStringLibrary.Conv_StringToDouble` (`|GetArrayItem` _returnvalue 5)) (`KismetStringLibrary.Conv_StringToDouble` (`|GetArrayItem` _returnvalue 6))))

(fn `SetupDevices`
  (returns (SetupComplete :type Boolean))
  ; First, check if Nuitrack Manager has been placed on this level
  (bind _outactors (`GameplayStatics.GetAllActorsOfClass` "/NuitrackPlugin/Blueprints/BP_NuitrackManager.BP_NuitrackManager_C"))
  (if (> (`KismetArrayLibrary.Array_Length` _outactors) 0)
    ; Then check for Kinect device
    (bind _returnvalue (`NuitrackUtils.GetDevices`))
    (if (> (`KismetArrayLibrary.Array_Length` _returnvalue) 0)
      (`KismetSystemLibrary.PrintString` "Nuitrack/Kinect setup complete" true true (struct :`R` 1.0 :`G` 1.0 :`B` 1.0 :`A` 1.0) 5.0)
      (return true)
      (else
        (`KismetSystemLibrary.PrintString` "Oops, Nuitrack device not found" true true (struct :`R` 1.0 :`G` 0.008761 :`A` 1.0) 10.0)))
    (else
      (`KismetSystemLibrary.PrintString` "Oops, Nuitrack Manager missing from level" true true (struct :`R` 1.0 :`G` 0.008761 :`A` 1.0) 10.0)))
  (return false))

(fn `SwapAxes`
  (params (RawEulerX :type "Float (double-precision)") (RawEulerY :type "Float (double-precision)") (RawEulerZ :type "Float (double-precision)"))
  (returns (EulerX :type "Float (double-precision)") (EulerY :type "Float (double-precision)") (EulerZ :type "Float (double-precision)"))
  (return (* RawEulerY 1.0) (* RawEulerZ -1.0) RawEulerX))

(fn `UnSnap`
  (params (InEulerX :type "Float (double-precision)") (InEulerY :type "Float (double-precision)") (InEulerZ :type "Float (double-precision)"))
  (returns (SmoothEulerX :type "Float (double-precision)") (SmoothEulerY :type "Float (double-precision)") (SmoothEulerZ :type "Float (double-precision)"))
  (return InEulerX InEulerY InEulerZ))

(fn `UserConstructionScript`)