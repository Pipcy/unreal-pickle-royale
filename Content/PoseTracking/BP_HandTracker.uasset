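; BP_HandTracker drives a Paddle actor from the player's right hand using Nuitrack body tracking.
; If a Nuitrack manager exists at BeginPlay, a looping timer runs UpdateHand at about 60 Hz.
; Each update reads the first user's hand joint and, above a confidence threshold, offsets it by Louis's location, swaps axes and moves the Paddle.
; Left-handed tracking is unimplemented; debug prints and a line remain.
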(event `self.ReceiveBeginPlay`
  ; init
  (bind _outactors (`GameplayStatics.GetAllActorsOfClass` "/NuitrackPlugin/Blueprints/BP_NuitrackManager.BP_NuitrackManager_C"))
  (if (> (`KismetArrayLibrary.Array_Length` _outactors) 0)
    ;; for now, we assume always right handed
    (set `self.isRightHanded` true)
    (set `self.jointConfidenceThreshhold` 0.2)
    ;; run the update event every 0.016 s = 60 Hz
    (`KismetSystemLibrary.K2_SetTimerDelegate` (delegate `UpdateHand`) 0.016 true true)
    (else
      (`KismetSystemLibrary.PrintString` "UH OH: no nuitrack manager found" true true (struct :`R` 1.0 :`B` 0.00746 :`A` 1.0) 10.0))))

(event `UpdateHand`
  (bind _returnvalue (`NuitrackUtils.GetUsers`))
  (`KismetSystemLibrary.PrintString` (`KismetStringLibrary.Concat_StrStr` "GetUsers length:" (`KismetStringLibrary.Conv_IntToString` (`KismetArrayLibrary.Array_Length` _returnvalue))) true true (struct :`G` 0.66 :`B` 1.0 :`A` 1.0) 0.1)
  (if (`self.isRightHanded`)
    (bind (_transform3d _projectionpos _confidence) (`NuitrackUtils.GetJoint` (`.skeleton` (break `NuitrackUser` (`|GetArrayItem` _returnvalue))) "JOINT_RIGHT_HAND"))
    (if (>= _confidence (`self.jointConfidenceThreshhold`))
      (bind _returnvalue_2 (`KismetMathLibrary.MakeVector` (* (.y (+ (* (.location _transform3d) (1.0 1.0 1.0)) (`SceneComponent.K2_GetComponentLocation` (`self.Louis`)))) -1.0) (.x (+ (* (.location _transform3d) (1.0 1.0 1.0)) (`SceneComponent.K2_GetComponentLocation` (`self.Louis`)))) (.z (+ (* (.location _transform3d) (1.0 1.0 1.0)) (`SceneComponent.K2_GetComponentLocation` (`self.Louis`))))))
      (`SceneComponent.K2_SetWorldLocation` (`self.paddle`) _returnvalue_2 false false)
      (`KismetSystemLibrary.DrawDebugLine` _returnvalue_2 (0.0 0.0 -1000.0) (`KismetMathLibrary.MakeColor` 200.0) 0.016 4.0)
      (else
        (`KismetSystemLibrary.PrintString` "oops")))
    (else
      (`KismetSystemLibrary.PrintString` "bad news bears, you're left handed"))))

(fn `UserConstructionScript`)