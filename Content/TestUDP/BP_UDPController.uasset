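; UDP controller that links a physical paddle to the game as an input device when keyboard mode is off.
; On start or settings updates, it applies the GameInstance IP and port, sends "gameplay", and marks pairing by whether data arrives within a timeout.
; Received bytes trigger Serving or Swing on the BP_Chub pawn.
; A looping monitor is set up to flag silence, unpair the paddle and broadcast connection loss.
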(event `self.ReceiveBeginPlay`
  (add `self.OnUpdateConnectionSettings` (delegate `CheckConnection`))
  (`self.CheckConnection`)
  (if (not (`/Game/UI/BP_GameInstance.Play Mode Keyboard?` (stale `CheckConnection` _asbp_game_instance)))
    (`KismetSystemLibrary.K2_SetTimerDelegate` (delegate `MonitorConnection`) 0.0 true true)))

(event `CheckConnection`
  (bind (_sendip _sendport _sendboundport _sendboundip _receiveip _receiveport _sendsocketname _receivesocketname _buffersize _bshouldautoopensend _bshouldautoopenreceive _bshouldopenreceivetoboundsendport _breceivedataongamethread) (break `UDPSettings` (`UDPComponent.Settings` (`self.UDP-paddle`))))
  ; if we are in paddle mode, then load the paddle ip & port from the gameinstance
  (`KismetSystemLibrary.PrintString` "checking connection..." true true (struct :`R` 1.0 :`G` 0.732426 :`A` 1.0) 10.0)
  (bind _asbp_game_instance (cast `/Game/UI/BP_GameInstance` (`GameplayStatics.GetGameInstance`))
    (:`then`
      (if (not (`/Game/UI/BP_GameInstance.Play Mode Keyboard?` _asbp_game_instance))
        ; if ip and port are still their defaults (assigned in Gamemode), we haven't paired yet
        (if (not (or (== (`/Game/UI/BP_GameInstance.PaddlePort` _asbp_game_instance) 1234) (`KismetStringLibrary.EqualEqual_StrStr` (`/Game/UI/BP_GameInstance.PaddleIP` _asbp_game_instance) "1.1.1.1")))
          ; if not the defaults, update the udp component settings
          (bind _asbp_game_instance_2 (cast `/Game/UI/BP_GameInstance` (`GameplayStatics.GetGameInstance`)))
          (bind _paddleip (`/Game/UI/BP_GameInstance.PaddleIP` _asbp_game_instance_2))
          (set `UDPComponent.Settings` (make `UDPSettings` _paddleip (`/Game/UI/BP_GameInstance.PaddlePort` _asbp_game_instance_2) _paddleip _receiveport _sendsocketname _receivesocketname _buffersize _bshouldautoopensend _bshouldautoopenreceive _bshouldopenreceivetoboundsendport _breceivedataongamethread) (`self.UDP-paddle`))
          (`KismetSystemLibrary.PrintString` "updated udp settings" true true (struct :`R` 1.0 :`G` 1.0 :`B` 1.0 :`A` 1.0) 5.0)
          (`self.SendStringToPaddle` "gameplay")
          ; attempt to listen for data
          (bind _returnvalue (`KismetSystemLibrary.K2_SetTimerDelegate` (delegate `AttemptConnection`) 0.1 true))
          (`KismetSystemLibrary.Delay` (`KismetMathLibrary.Conv_IntToDouble` (`self.PaddleTimeoutSeconds`)))
          (`KismetSystemLibrary.K2_ClearAndInvalidateTimerHandle` _returnvalue)
          (`KismetSystemLibrary.PrintString` (`KismetStringLibrary.Concat_StrStr` "is receiving: " (`KismetStringLibrary.Conv_BoolToString` (`self.isReceiving`))) true true (struct :`R` 0.08356 :`G` 1.0 :`A` 1.0) 10.0)
          ; if we are receiving data from the inputted ip and port, we are paired :)
          (bind _asbp_game_instance_3 (cast `/Game/UI/BP_GameInstance` (`GameplayStatics.GetGameInstance`)))
          (set `/Game/UI/BP_GameInstance.PaddleIsPaired` (`self.isReceiving`) _asbp_game_instance_3)
          (else
            (set `/Game/UI/BP_GameInstance.PaddleIsPaired` false _asbp_game_instance)
            (`KismetSystemLibrary.PrintString` "ERROR: paddle info is defaults" true true (struct :`R` 1.0 :`B` 0.00868 :`A` 1.0) 10.0)))
        (else
          (`KismetSystemLibrary.PrintString` "keyboard mode" true true (struct :`R` 1.0 :`G` 1.0 :`B` 1.0 :`A` 1.0) 5.0))))
    (:`CastFailed`
      (`KismetSystemLibrary.PrintString` "ERROR: BP_UDPController failed to cast game instance" true true (struct :`R` 1.0 :`B` 0.035682 :`A` 1.0) 10.0))))

(event `AttemptConnection`
  ; attempt to listen for data
  (set `self.isReceiving` (< (- (`GameplayStatics.GetRealTimeSeconds`) (`self.LastReceiveTime`)) 1.0)))

(event `self.UDP-paddle.OnReceivedBytes`
  (params (Bytes :type "Array of Byte (by ref)") (IPAddress :type String) (Port :type "Integer (by ref)"))
  (bind _returnvalue (`CUBlueprintLibrary.Conv_BytesToString` Bytes))
  (bind _returnvalue_2 (`GameplayStatics.GetPlayerPawn` 0))
  ; on receive bytes via UDP
  (`KismetSystemLibrary.PrintString` "receiving" true true (struct :`R` 0.572917 :`G` 0.572917 :`B` 0.572917 :`A` 1.0) 0.5)
  (set `self.ReceivedBytes` Bytes)
  (if (not (`/Game/UI/BP_GameInstance.Play Mode Keyboard?` (stale `CheckConnection` _asbp_game_instance)))
    (set `self.LastReceiveTime` (`GameplayStatics.GetRealTimeSeconds`))
    (`KismetSystemLibrary.PrintString` _returnvalue)
    (if (== _returnvalue "detect btn push")
      (bind _asbp_chub (cast `/Game/Player/Chub/BP_Chub` _returnvalue_2))
      (`/Game/Player/Chub/BP_Chub.serving` _asbp_chub)
      (else
        (bind _asbp_chub_2 (cast `/Game/Player/Chub/BP_Chub` _returnvalue_2))
        (`/Game/Player/Chub/BP_Chub.swing` _asbp_chub_2)))))

(event `MonitorConnection`
  ; check that we are still receiving data
  (if (> (- (`GameplayStatics.GetRealTimeSeconds`) (`self.LastReceiveTime`)) (`self.PaddleTimeoutSeconds`))
    ; if no data for the duration of the timeout, notify pause/settings WB that connection was lost
    (`self.OnConnectionLost`)
    (set `self.isReceiving` false)
    (bind _asbp_game_instance (cast `/Game/UI/BP_GameInstance` (`GameplayStatics.GetGameInstance`)))
    (set `/Game/UI/BP_GameInstance.PaddleIsPaired` false _asbp_game_instance)
    (`KismetSystemLibrary.PrintString` "UDPController: Connection loss detected!" true true (struct :`R` 1.0 :`G` 0.182528 :`B` 0.05277 :`A` 1.0) 10.0)))

(fn `GetArrayAverage`
  (params (input_array :type "Array of Float (double-precision)"))
  (returns (average :type "Float (double-precision)"))
  (locals (total_sum :type "Float (double-precision)") (input_array_L :type "Array of Float (double-precision)"))
  (set `local.input_array_L` input_array)
  (set `local.total_sum` 0.0)
  (if (== (`KismetArrayLibrary.Array_Length` (`local.input_array_L`)) 0)
    (`KismetSystemLibrary.PrintString` "UH OH: divide by 0" true true (struct :`R` 0.804688 :`G` 0.148283 :`A` 1.0) 0.5)
    (return 0.0)
    (else
      (for _array_element (`local.input_array_L`)
        (set `local.total_sum` (+ _array_element (`local.total_sum`))))
      (return (/ (`local.total_sum`) (`KismetArrayLibrary.Array_Length` (`local.input_array_L`)))))))

(fn `SendStringToPaddle`
  (params (SendString :type String))
  (`UDPComponent.EmitBytes` (`self.UDP-paddle`) (`CUBlueprintLibrary.Conv_StringToBytes` SendString)))

(fn `UserConstructionScript`)