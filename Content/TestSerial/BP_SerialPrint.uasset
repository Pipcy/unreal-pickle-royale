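; Test actor that rotates the BP_Paddle3 actor from orientation data streamed by an Arduino over a serial COM port.
; BeginPlay opens the port and finds the paddle, then a self-recalling Delay loop reads and prints each line.
; Three-value comma-separated lines become a target rotation that the paddle eases toward with RInterpTo.
; EndPlay closes the port; a VaRest JSON object is created, but its parsing is disconnected.
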(event `self.ReceiveBeginPlay`
  (bind (_bopened _returnvalue) (`SerialCom.OpenComPort` 3 115200))
  (if _bopened
    (set `self.arduino` _returnvalue)
    (bind _returnvalue_2 (`GameplayStatics.GetActorOfClass` "/Game/Assets/paddle3/BP_Paddle3.BP_Paddle3_C"))
    (set `self.Paddle` _returnvalue_2)
    (bind _returnvalue_3 (`VaRestSubsystem.ConstructVaRestJsonObject` (subsystem `VaRestSubsystem`)))
    (set `self.JsonObject` _returnvalue_3)
    (`self.ReadSerialLineLoop`)
    (else
      (`KismetSystemLibrary.PrintString` "port not open"))))

(event `ReadSerialLineLoop`
  (bind (_bsuccess _returnvalue) (`SerialCom.Readln` (`self.arduino`)))
  (`KismetSystemLibrary.PrintString` _returnvalue true true (struct :`R` 1.0 :`B` 0.11183 :`A` 1.0))
  (bind _returnvalue_2 (`KismetStringLibrary.ParseIntoArray` _returnvalue ","))
  (if (== (`KismetArrayLibrary.Array_Length` _returnvalue_2) 3)
    (bind _result (`/Engine/EditorBlueprintResources/StandardMacros.NegateFloat` (`KismetStringLibrary.Conv_StringToDouble` (`|GetArrayItem` _returnvalue_2 1)))
      (:`  `
        (bind _result_2 (`/Engine/EditorBlueprintResources/StandardMacros.NegateFloat` (`KismetStringLibrary.Conv_StringToDouble` (`|GetArrayItem` _returnvalue_2 2)))
          (:`  `
            (bind _output_get (set `self.TargetRotation` (`KismetMathLibrary.MakeRotator` _result _result_2 (`KismetStringLibrary.Conv_StringToDouble` (`|GetArrayItem` _returnvalue_2)))))
            (`self.K2_SetActorRotation` (`self.Paddle`) (`KismetMathLibrary.RInterpTo` (`self.K2_GetActorRotation` (`self.Paddle`)) _output_get (`GameplayStatics.GetWorldDeltaSeconds`) 5.0) false)
            (`KismetSystemLibrary.Delay` 0.001)
            (`self.ReadSerialLineLoop`)))))
    (else
      (`KismetSystemLibrary.Delay` 0.001)
      (`self.ReadSerialLineLoop`))))

(event `self.ReceiveEndPlay`
  (params (EndPlayReason :type "EEndPlayReason Enum" :default "Destroyed"))
  (bind _arduino (`self.arduino`))
  (`/Engine/EditorBlueprintResources/StandardMacros.IsValid` _arduino
    (:`Is Valid`
      (`SerialCom.Close` _arduino))))

(fn `UserConstructionScript`)