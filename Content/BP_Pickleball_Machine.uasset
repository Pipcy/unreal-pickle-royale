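; Pickleball ball machine that, if switched on at BeginPlay, repeatedly launches balls at random spots in a chosen B-side service area.
; Each toss moves the goal post mesh within that court box, then solves an arc velocity to it, using doubled gravity when a player character exists.
; The spawned BP_Ball_Projectile is announced through OnBallSpawnedByPballMachine for the opponent AI, then destroyed after a delay before the next toss.
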(event `self.ReceiveBeginPlay`
  (`KismetSystemLibrary.Delay` 3.0) ; allow the janky set up to get the timing right with goalpost movement
  (if (`self.Machine On / Off`)
    (`self.TossBall`)))

(event `UpdateGoalPost`
  (bind (_feeding_box_extent_x _feeding_box_extent_y) (`KismetMathLibrary.BreakVector` (`self.Feeding Box Extent`)))
  (bind _returnvalue (`KismetMathLibrary.RandomPointInBoundingBox` (`self.Pickleball Machine Ball Feeding Location`) (`KismetMathLibrary.MakeVector` _feeding_box_extent_x _feeding_box_extent_y)))
  ; update landing goal post
  (bind _returnvalue_2 (`GameplayStatics.GetActorOfClass` "/Game/BP_courtSimple.BP_courtSimple_C"))
  (switch `/Game/Opponents/AI/Anthony/Enums/Enum_CourtAreas` (`self.Enum Court Areas`)
    (:`NewEnumerator4`
      (bind _bservicearea (`/Game/BP_courtSimple.BServiceArea` _returnvalue_2))
      (set `self.Pickleball Machine Ball Feeding Location` (`SceneComponent.K2_GetComponentLocation` _bservicearea))
      (set `self.Feeding Box Extent` (`BoxComponent.GetScaledBoxExtent` _bservicearea)))
    (:`NewEnumerator5`
      (bind _bservicearealeft (`/Game/BP_courtSimple.BServiceAreaLeft` _returnvalue_2))
      (set `self.Pickleball Machine Ball Feeding Location` (`SceneComponent.K2_GetComponentLocation` _bservicearealeft))
      (set `self.Feeding Box Extent` (`BoxComponent.GetScaledBoxExtent` _bservicearealeft)))
    (:`NewEnumerator6`
      (bind _bservicearearight (`/Game/BP_courtSimple.BServiceAreaRight` _returnvalue_2))
      (set `self.Pickleball Machine Ball Feeding Location` (`SceneComponent.K2_GetComponentLocation` _bservicearearight))
      (set `self.Feeding Box Extent` (`BoxComponent.GetScaledBoxExtent` _bservicearearight))))
  (`SceneComponent.K2_SetWorldLocation` (`self.GoalPost Mesh`) _returnvalue false false)
  (`KismetSystemLibrary.PrintString` (`KismetStringLibrary.Concat_StrStr` "Current Goal Position: " (`KismetStringLibrary.Conv_VectorToString` _returnvalue))))

(event `TossBall`
  (bind _returnvalue (`SceneComponent.K2_GetComponentLocation` (`self.BallSpawnLocationREF`)))
  ; toss the ball to a specified location
  (`self.UpdateGoalPost`)
  (`KismetSystemLibrary.Delay` 1.0)
  (`KismetSystemLibrary.PrintString` "Ball Machine toss ball")
  (bind _balllandingposition (`self.SetBallLandingPosition`))
  (bind (_gravityoverride _gravityscale) (`self.SetGravityOverrideandScale`))
  (bind _outlaunchvelocity (`GameplayStatics.SuggestProjectileVelocity_CustomArc` _returnvalue _balllandingposition _gravityoverride)) ; make projectile from pickleball machine feeder head to the goal post location
  (bind _returnvalue_2 (`|SpawnActorFromClass` "/Game/BP_Ball_Projectile.BP_Ball_Projectile_C" (`KismetMathLibrary.Conv_VectorToTransform` _returnvalue) "Undefined" "MultiplyWithRoot" null _outlaunchvelocity _gravityscale _balllandingposition (struct :`TagName` "Ball.HeadingTo.Bside") null)) ; add UI to modularly set this (ball heading)
  (`self.On Ball Spawned by Pball Machine` _returnvalue_2) ; this is caslling on AIC_NPC_Opponent
  (`KismetSystemLibrary.Delay` 5.0)
  (`self.K2_DestroyActor` _returnvalue_2)
  (`KismetSystemLibrary.Delay` 2.0)
  (`self.TossBall`))

(fn `SetBallLandingPosition`
  (returns (BallLandingPosition :type "Vector Structure"))
  (locals (Local_BallLandingPosition :type "Vector Structure"))
  (set `local.Local_BallLandingPosition` (`SceneComponent.K2_GetComponentLocation` (`self.GoalPost Mesh`)))
  (return (`local.Local_BallLandingPosition`)))

(fn `SetGravityOverrideandScale`
  (returns (GravityOverride :type "Float (double-precision)") (GravityScale :type "Float (double-precision)"))
  (locals (Local_GravityOverride :type "Float (double-precision)" :default 0.0) (Local_GravityScale :type "Float (double-precision)" :default 0.0))
  (bind _returnvalue (`GameplayStatics.GetPlayerCharacter` 0))
  (bind _charactermovement (`Character.CharacterMovement` _returnvalue))
  (`/Engine/EditorBlueprintResources/StandardMacros.IsValid` _returnvalue
    (:`Is Valid`
      (set `local.Local_GravityOverride` (* (/ (`MovementComponent.GetGravityZ` _charactermovement) (`CharacterMovementComponent.GravityScale` _charactermovement)) 2.0))
      (set `local.Local_GravityScale` 2.0))
    (:`Is Not Valid`
      (set `local.Local_GravityOverride` 0.0)
      (set `local.Local_GravityScale` 1.0)))
  (return (`local.Local_GravityOverride`) (`local.Local_GravityScale`)))

(fn `UserConstructionScript`)