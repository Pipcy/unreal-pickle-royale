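; Player controller for a practice project that registers the Enhanced Input mapping context and toggles a pause menu.
; BeginPlay adds IMC_practice to the local player's input subsystem.
; IA_PauseGame flips IsPausedMenuOpen, creating or removing the WB_pause widget while switching input mode, mouse cursor visibility and game pause state.
; A fresh widget is created on each open rather than reused.
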(event `self.ReceiveBeginPlay`
  ; hook up the new input mapping context
  (`EnhancedInputSubsystemInterface.AddMappingContext` (pcsubsystem `EnhancedInputLocalPlayerSubsystem` (`GameplayStatics.GetPlayerController` 0)) "/Game/UI/inputs/IMC_practice.IMC_practice" 0 (struct)))

(event `EnhancedInput|/Game/UI/inputs/Actions/IA_PauseGame`
  (params (ActionValue :type Boolean) (ElapsedSeconds :type "Float (double-precision)") (TriggeredSeconds :type "Float (double-precision)") (InputAction :type "InputAction Object Reference" :default "/Game/UI/inputs/Actions/IA_PauseGame.IA_PauseGame"))
  (bind _returnvalue (`GameplayStatics.GetPlayerController` 0))
  (bind _returnvalue_2 (`GameplayStatics.GetPlayerController` 0))
  ; pausing/un-pausing game by hitting P
  (:`Started`
    (if (not (`self.isPausedMenuOpen?`))
      (set `self.isPausedMenuOpen?` true)
      (bind _returnvalue_3 (`|CreateWidget` "/Game/UI/WB_pause.WB_pause_C" _returnvalue_2))
      (bind _output_get (set `self.PauseMenuWidget` _returnvalue_3))
      (`UserWidget.AddToViewport` _output_get 0)
      (`WidgetBlueprintLibrary.SetInputMode_GameAndUIEx` _returnvalue_2 (`self.PauseMenuWidget`))
      (set `PlayerController.bShowMouseCursor` true (`GameplayStatics.GetPlayerController` 0))
      (`GameplayStatics.SetGamePaused` true)
      (else
        (set `self.isPausedMenuOpen?` false)
        (`WidgetBlueprintLibrary.SetInputMode_GameOnly` _returnvalue)
        (set `PlayerController.bShowMouseCursor` false _returnvalue)
        (`Widget.RemoveFromParent` (`self.PauseMenuWidget`))
        (`GameplayStatics.SetGamePaused` false)))))

(fn `UserConstructionScript`)