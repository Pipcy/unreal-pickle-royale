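; BP_GameBase2 runs a practice game that launches balls on a repeating cycle and tracks score and misses.
; BeginPlay adds the BP_UI_Practice widget to the viewport, then starts SpawnBall, which spawns and impulses a BP_Ball.
; After timed delays it checks BallHit, zeroes Score and sets a miss message on failure, destroys the ball and calls itself again.
; The score increment and player-location capture are disconnected, and BallHit is only cleared here.
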(event `self.ReceiveTick`
  (params (DeltaSeconds :type "Float (single-precision)")))

(event `self.ReceiveBeginPlay`
  (`KismetSystemLibrary.PrintString` "fired")
  (bind _returnvalue (`|CreateWidget` "/Game/Levels/BP_UI_Practice.BP_UI_Practice_C"))
  (bind _output_get (set `self.UI Widget` _returnvalue))
  (`UserWidget.AddToViewport` _output_get 0)
  (`self.SpawnBall`))

(event `SpawnBall`
  ; spawn a ball every X second and then destroy
  (`KismetSystemLibrary.PrintString` (`KismetStringLibrary.Conv_IntToString` (`self.Score`)))
  (bind _returnvalue (`|SpawnActorFromClass` "/Game/BP_Ball.BP_Ball_C" (`self.Spawn Transform`) "Undefined" "MultiplyWithRoot" null (0.0 0.0 0.0) 1.0 null))
  (`PrimitiveComponent.AddImpulse` (`/Game/BP_Ball.Sphere` _returnvalue) (-100.0 0.0 30.0) "None" false)
  (`KismetSystemLibrary.Delay` 3.0)
  ; check/update score
  (if (not (`self.Ball Hit?`))
    (set `self.Score` 0)
    (`KismetSystemLibrary.PrintString` "ball did not hit")
    (set `self.UI Message Text` "YOU MISSED"))
  (`KismetSystemLibrary.Delay` 2.0)
  (set `self.UI Message Text` "")
  (`self.K2_DestroyActor` _returnvalue)
  (set `self.Ball Hit?` false)
  (`self.SpawnBall`))

(event `Reset Game`
  (set `self.Score` 0))

(fn `UserConstructionScript`)