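; BP_GamePractice is a practice-mode game Blueprint for a ball game, handling serving, bounce counting and score reset.
; SimplePlayerServe spawns a BP_Ball beside the player and launches it with an impulse; DestoryBall removes it after a delay.
; CheckandUpdate logs and increments the bounce count, flagging repeat bounces.
; The looping SpawnBall physics-ball launcher is marked deprecated, and the hit/miss scoring and message logic is disconnected.
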(event `self.ReceiveBeginPlay`)

(event `SpawnBall`
  ;[0.15 0.09387 0.04088 0.5] spawn a ball every X second and then destroy -> deprecated!!
  (`KismetSystemLibrary.PrintString` "Spawn Ball")
  (bind _returnvalue (`|SpawnActorFromClass` "/Game/BP_Ball_Physics.BP_Ball_Physics_C" (`self.Spawn Transform`) "Undefined" "MultiplyWithRoot" null (0.0 0.0 0.0) 0.0 null))
  (`PrimitiveComponent.AddImpulse` (`/Game/BP_Ball_Physics.Sphere` _returnvalue) (-1800.0 0.0 600.0) "None" false)
  (`KismetSystemLibrary.Delay` 3.0)
  (`self.K2_DestroyActor` _returnvalue)
  (set `self.Ball Hit?` false)
  (set `self.Bounce Number` 0)
  (`self.SpawnBall`))

(event `Check and Update`
  (params (BouncedZone :type Boolean))
  (`KismetSystemLibrary.PrintString` "check fired")
  (if (not (== (`self.Bounce Number`) 0))
    (`KismetSystemLibrary.PrintString` "Bounce twice! "))
  (`KismetSystemLibrary.PrintString` (`KismetStringLibrary.Concat_StrStr` "BP_GamePractice: Bounce number: " (`KismetStringLibrary.Conv_IntToString` (`self.Bounce Number`))))
  (`/Engine/EditorBlueprintResources/StandardMacros.IncrementInt` (`self.Bounce Number`)))

(event `Reset Game`
  (set `self.Score` 0))

(event `SimplePlayerServe`
  ; Serve ball
  ;; set and store player location
  (bind _output_get (set `self.PlayerLocation` (`self.K2_GetActorLocation` (`GameplayStatics.GetPlayerCharacter` 0))))
  (`KismetSystemLibrary.PrintString` "Spawn Ball")
  (bind _returnvalue (`|SpawnActorFromClass` "/Game/BP_Ball.BP_Ball_C" (`KismetMathLibrary.MakeTransform` (`KismetMathLibrary.MakeVector` (.x _output_get) (+ (.y _output_get) 50.0) (.z _output_get))) "Undefined" "MultiplyWithRoot" null (0.0 0.0 0.0) 1.0 null))
  (`PrimitiveComponent.AddImpulse` (`/Game/BP_Ball.Sphere` _returnvalue) (120.0 0.0 45.0) "None" false))

(event `DestoryBall`
  ; Serve ball
  (`KismetSystemLibrary.Delay` 3.0)
  (`self.K2_DestroyActor` (stale `SimplePlayerServe` _returnvalue)))

(fn `UserConstructionScript`)