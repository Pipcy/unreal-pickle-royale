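; Game mode for a pickleball-style match, PVE or local two-player, played until a side reaches the target score.
; BeginPlay resets scores, signals the UDP paddle controller, binds player events and plays an intro sequence before the first serve.
; Ball bounce and hit events drive gameplay-tag rules for short and out balls, with only the serving side able to score.
; A win plays an ending sequence, saves results to the GameInstance and opens the end level.
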(event `self.ReceiveBeginPlay`
  (bind _player_ref (`self.Player Ref`))
  ; set score to 0
  (set `self.player score` 0)
  (set `self.opponent score` 0)
  (`self.send string to paddle` "gameplay")
  ; game instance ref
  (bind _asbp_game_instance (cast `/Game/UI/BP_GameInstance` (`GameplayStatics.GetGameInstance`))
    (:`then`
      (bind _output_get (set `self.Game Instance Ref` _asbp_game_instance))
      (set `/Game/UI/BP_GameInstance.Player Score` 0 _output_get)
      (set `/Game/UI/BP_GameInstance.Enemy Score` 0 _output_get)
      (set `/Game/UI/BP_GameInstance.points` 0 _output_get)
      ; set up the air zone check BP
      (bind _returnvalue (`GameplayStatics.GetActorOfClass` "/Game/BP_CourtAreaInAir.BP_CourtAreaInAir_C"))
      (set `self.Ball In Air Zone Ref` _returnvalue)
      ; register player(s)
      ;; get player ref
      (bind _asbp_chub (cast `/Game/Player/Chub/BP_Chub` (`Controller.K2_GetPawn` (`GameplayStatics.GetPlayerController` 0)))
        (:`then`
          (set `self.Player Ref` _asbp_chub)
          (add `/Game/Player/Chub/BP_Chub.On Player Served` _player_ref (`|CreateDelegate` :!event `Handle Player Served`))
          (add `/Game/Player/Chub/BP_Chub.On Player Points Updated` _player_ref (`|CreateDelegate` :!event `Update Player Points`))
          (if (`/Game/UI/BP_GameInstance.PVE?` (`self.Game Instance Ref`))
            ;; PVE - get Opponent ref
            (bind _returnvalue_2 (`GameplayStatics.GetActorOfClass` "/Game/Opponents/AI/Anthony/BP_NPC_Opponent.BP_NPC_Opponent_C"))
            (set `self.Opponent Character Ref` _returnvalue_2)
            ; level sequence
            (bind (_outactor _returnvalue_3) (`LevelSequencePlayer.CreateLevelSequencePlayer` "/Game/Camera_Sequences/NewLevelSequence.NewLevelSequence" :!label _label))
            (`MovieSceneSequencePlayer.Play` (`LevelSequenceActor.SequencePlayer` _outactor))
            (add `MovieSceneSequencePlayer.OnFinished` _returnvalue_3 (delegate `On Finish Playing Start Sequence`))
            (else
              ;; PVP - get player 1 ref
              (bind _returnvalue_4 (`GameplayStatics.CreatePlayer` 1))
              (bind _asbp_chub_2 (cast `/Game/Player/Chub/BP_Chub` (`Controller.K2_GetPawn` _returnvalue_4))
                (:`then`
                  (bind _output_get_2 (set `self.player 1 Ref` _asbp_chub_2))
                  (add `/Game/Player/Chub/BP_Chub.On Player Served` _output_get_2 (`|CreateDelegate` :!event `Handle Player Served`))
                  (add `/Game/Player/Chub/BP_Chub.On Player Points Updated` (`self.player 1 Ref`) (`|CreateDelegate` :!event `Update Player Points`))
                  (goto _label))
                (:`CastFailed`
                  (`KismetSystemLibrary.PrintString` "Hello"))))))
        (:`CastFailed`
          (`KismetSystemLibrary.PrintString` "Hello"))))
    (:`CastFailed`
      (`KismetSystemLibrary.PrintString` "Hello"))))

(event `UpdateBallRef`
  (params (`Spawned Ball Ref` :type "/Game/BP_Ball_Projectile Object Reference"))
  ; when a new ball spawn (by either player or opponent) register
  (set `self.current ball ref` `Spawned Ball Ref`)
  (add `/Game/BP_Ball_Projectile.On Ball Overlap Court Area` (`self.current ball ref`) (`|CreateDelegate` :!event `Handle On Ball Overlapped Court Area`))
  (add `/Game/BP_Ball_Projectile.On Ball Overlap Something Else` (`self.current ball ref`) (`|CreateDelegate` :!event `On Ball Overlapped Something Else`))
  (add `/Game/BP_Ball_Projectile.On Ball Hit Event Triggered` (`self.current ball ref`) (`|CreateDelegate` :!event `On Ball Hit Event Triggered`)))

(event `Increment Player Score`
  ; score management
  ;; Increment Player Score
  (`/Engine/EditorBlueprintResources/StandardMacros.IncrementInt` (`self.player score`)
    (:`  `
      (`self.print score`) ; temporary
      (`self.Queue Pop Up Text` "Score!")
      (set `self.Player can Serve?` true)
      (`self.On Player Score Updated` (`self.player score`)) ; observed by PC_IntegratedBasicUI
    )))

(event `Match Loop`
  ; Main Match Loop
  (`self.player's Turn to Serve`))

(event `player's Turn to Serve`
  ; Main Match Loop
  (set `self.TurnToServe` (struct :`TagName` "TurnToServe.Player")) ; begin with Player Serve
  (set `self.Player can Serve?` true)
  (`self.Queue Pop Up Text` "Hold 6 or Button to Serve."))

(event `Increment Opponent Score`
  ; score management
  ;; Increment Opponent Score
  (`/Engine/EditorBlueprintResources/StandardMacros.IncrementInt` (`self.opponent score`)
    (:`  `
      (`self.print score`) ; temporary
      (`self.Queue Pop Up Text` "Opponent Scored!")
      (`self.On Opponent Score Updated` (`self.opponent score`)) ; observed by PC_IntegratedBasicUI
    )))

(event `Enemy's Turn to Serve`
  ; Main Match Loop
  (set `self.TurnToServe` (struct :`TagName` "TurnToServe.Opponent")) ; begin with Player Serve
  (`self.Queue Pop Up Text` "Opponents turn to serve")
  (`self.Opponent Serve`))

(event `Handle On Ball Overlapped Court Area`
  (params (`Other Comp` :type "PrimitiveComponent Object Reference"))
  ; Main Match Loop
  (`KismetSystemLibrary.PrintString` (`KismetStringLibrary.Concat_StrStr` "BALL HIT COURT AREA: " (`KismetSystemLibrary.GetDisplayName` `Other Comp`)) false false (struct :`R` 0.106177 :`G` 1.0 :`A` 1.0))
  (`self.On Bounce Info Updated`))

(event `On Ball Hit Event Triggered`
  (params (`other comp` :type "PrimitiveComponent Object Reference"))
  ; Main Match Loop
  (if (`/Game/BP_Ball_Projectile.ball is Active?` (`self.current ball ref`))
    (`KismetSystemLibrary.PrintString` (`KismetSystemLibrary.GetDisplayName` `other comp`) false false)
    (if (and (`ActorComponent.ComponentHasTag` `other comp` "floor plane") (not (`/Game/BP_CourtAreaInAir.Ball in Court Air Zone?` (`self.Ball In Air Zone Ref`))))
      (`KismetSystemLibrary.PrintString` "Hello" false false)
      (`self.Handle Ball Out`) ; update score  based on rules
    )
    (else
      (`KismetSystemLibrary.PrintString` "Hello" false false))))

(event `print score`
  ; score management
  ;; temp - print score
  (`KismetSystemLibrary.PrintString` (`KismetStringLibrary.Concat_StrStr` "Player:  " (`KismetStringLibrary.Conv_IntToString` (`self.player score`)) "Opponent: " (`KismetStringLibrary.Conv_IntToString` (`self.opponent score`)))))

(event `Update Player Points`
  (params (`Player Point Increment` :type Integer))
  (bind _game_instance_ref (`self.Game Instance Ref`))
  ; score management
  ;; update player points in the game instance (called by event dispatchered in chub BP)
  (set `/Game/UI/BP_GameInstance.points` (+ (`/Game/UI/BP_GameInstance.points` _game_instance_ref) `Player Point Increment`) _game_instance_ref))

(event `On Ball Overlapped Something Else`
  (params (`Other Comp` :type "PrimitiveComponent Object Reference"))
  ; Main Match Loop
  (`KismetSystemLibrary.PrintString` (`KismetStringLibrary.Concat_StrStr` "BALL HIT SOMETHING ELSE" (`KismetSystemLibrary.GetDisplayName` `Other Comp`)) true true (struct :`R` 1.0 :`G` 0.157706 :`A` 1.0)))

(event `On Finish Playing Start Sequence`
  ; level sequence
  (`self.Match Loop`))

(event `Opponent Serve`
  ; Main Match Loop
  ;; observed by Eval Match state
  (`self.On Opponent Serve Commanded`))

(event `Handle Player Served`
  ; Main Match Loop
  (`self.On Player Served`) ; listened by eval match state, change enemy motivation
)

(event `Player Win`
  ; score management
  ;; player win
  (`self.Queue Pop Up Text` "VICTORY")
  (set `/Game/UI/BP_GameInstance.player win?` true (`self.Game Instance Ref`))
  (`self.Go To Game End` :!label _label_2))

(event `On Bounce Info Updated`
  (bind _current_ball_ref (`self.current ball ref`))
  (bind _current_ball_ref_2 (`self.current ball ref`))
  (bind _most_recent_bounce_area (`/Game/BP_Ball_Projectile.Most Recent Bounce Area` _current_ball_ref_2))
  (bind _second_most_recent_bounce_area (`/Game/BP_Ball_Projectile.Second Most Recent Bounce Area` _current_ball_ref_2))
  ; check the rules based on bounce updates
  (`|SwitchGameplayTag` (`/Game/BP_Ball_Projectile.Ball Heading State` _current_ball_ref_2)
    (:`Ball.HeadingTo.Aside`
      (switch `/Game/Opponents/AI/Anthony/Enums/Enum_CourtAreas` _most_recent_bounce_area
        (:`NewEnumerator1`
          (switch `/Game/Opponents/AI/Anthony/Enums/Enum_CourtAreas` _second_most_recent_bounce_area :!label _label_3
            (:`NewEnumerator1`
              (`KismetSystemLibrary.PrintString` "player didn't make the ball pass the net (A side short)" false false (struct :`R` 1.0 :`B` 0.085713 :`A` 1.0) :!label _label_4)
              (`|SwitchGameplayTag` (`self.TurnToServe`)
                (:`TurnToServe.Player`
                  (`self.Enemy's Turn to Serve` :!label _label_5))
                (:`TurnToServe.Opponent`
                  (`self.Increment Opponent Score`)
                  (bind _somebody_won_ (`self.Check Win Condition`))
                  (if _somebody_won_
                    _
                    (else
                      (goto _label_5)))))
              (set `/Game/BP_Ball_Projectile.ball is Active?` false _current_ball_ref :!label _label_6)
              (`/Game/BP_Ball_Projectile.Set Ball Heading State` _current_ball_ref (struct :`TagName` "Ball.HeadingTo.Nowhere")))
            (:`NewEnumerator2`
              (goto _label_4))
            (:`NewEnumerator5`
              (`KismetSystemLibrary.PrintString` "good" false false (struct :`R` 0.036935 :`G` 1.0 :`A` 1.0) :!label _label_7))
            (:`NewEnumerator6`
              (goto _label_7))
            (:`NewEnumerator7`
              (goto _label_7))
            (:`NewEnumerator8`
              (goto _label_7))
            (:`NewEnumerator9`
              (goto _label_4))))
        (:`NewEnumerator2`
          (goto _label_3))
        (:`NewEnumerator5`
          (`KismetSystemLibrary.PrintString` "Opponent didn't make the ball pass the net (B side short)" false false (struct :`R` 1.0 :`G` 0.114338 :`B` 0.134234 :`A` 1.0) :!label _label_8)
          (`|SwitchGameplayTag` (`self.TurnToServe`)
            (:`TurnToServe.Player`
              (`self.Increment Player Score`)
              (bind _somebody_won__2 (`self.Check Win Condition`))
              (if _somebody_won__2
                (goto _label_6)
                (else
                  _)))
            (:`TurnToServe.Opponent`
              _))
          (`self.player's Turn to Serve`)
          (goto _label_6))
        (:`NewEnumerator6`
          (goto _label_8))
        (:`NewEnumerator8`
          (goto _label_8))
        (:`NewEnumerator9`
          (goto _label_3))))
    (:`Ball.HeadingTo.Bside`
      (switch `/Game/Opponents/AI/Anthony/Enums/Enum_CourtAreas` _most_recent_bounce_area ; opponent hit but ball bounce on B again
        (:`NewEnumerator1`
          (goto _label_4))
        (:`NewEnumerator2`
          (goto _label_4))
        (:`NewEnumerator5`
          _)
        (:`NewEnumerator6`
          _)
        (:`NewEnumerator8`
          _)
        (:`NewEnumerator9`
          (goto _label_4)))
      (switch `/Game/Opponents/AI/Anthony/Enums/Enum_CourtAreas` _second_most_recent_bounce_area
        (:`NewEnumerator1`
          _)
        (:`NewEnumerator2`
          _)
        (:`NewEnumerator5`
          (goto _label_8))
        (:`NewEnumerator6`
          (goto _label_8))
        (:`NewEnumerator7`
          _)
        (:`NewEnumerator8`
          (goto _label_8))
        (:`NewEnumerator9`
          _))
      (`KismetSystemLibrary.PrintString` "good" false false (struct :`R` 0.081203 :`G` 1.0 :`A` 1.0)))))

(event `Opponent Win`
  ; score management
  ;; Opponent win
  (`self.Queue Pop Up Text` "DEFEAT")
  (set `/Game/UI/BP_GameInstance.player win?` false (`self.Game Instance Ref`))
  (goto _label_2))

(event `Go To Game End`
  ; to to game end
  (bind (_outactor _returnvalue) (`LevelSequencePlayer.CreateLevelSequencePlayer` "/Game/Camera_Sequences/End_Play_Seq.End_Play_Seq"))
  (`MovieSceneSequencePlayer.Play` (`LevelSequenceActor.SequencePlayer` _outactor))
  (add `MovieSceneSequencePlayer.OnFinished` _returnvalue (delegate `On Finished Playing Ending Sequence`)))

(event `On Finished Playing Ending Sequence`
  (bind _game_instance_ref (`self.Game Instance Ref`))
  ; to to game end
  (set `/Game/UI/BP_GameInstance.Player Score` (`self.player score`) _game_instance_ref)
  (set `/Game/UI/BP_GameInstance.Enemy Score` (`self.opponent score`) _game_instance_ref)
  (`GameplayStatics.OpenLevelBySoftObjectPtr` "/Game/Levels/GameEnd/LevelGameEnd.LevelGameEnd"))

(fn `Check Win Condition`
  (returns (`Somebody Won?` :type Boolean))
  ; win condition
  (if (== (`self.player score`) (`self.Play to (Score)`))
    (`self.Player Win`)
    (return true)
    (elif (== (`self.opponent score`) (`self.Play to (Score)`))
      (`self.Opponent Win`)
      (return true)
      (else
        (return false)))))

(fn `Handle Ball Out`
  (bind _ball_heading_state (`/Game/BP_Ball_Projectile.Ball Heading State` (`self.current ball ref`)))
  (set `/Game/BP_Ball_Projectile.ball is Active?` false (`self.current ball ref`))
  (`KismetSystemLibrary.PrintString` "OUT" false false (struct :`R` 1.0 :`G` 0.268976 :`B` 0.966077 :`A` 1.0))
  (if (< (`/Game/BP_Ball_Projectile.Ball Bounce Count` (`self.current ball ref`)) 1)
    (`|SwitchGameplayTag` _ball_heading_state ; ball is out
      (:`Ball.HeadingTo.Aside`
        (`self.player's Turn to Serve` :!label _label) ; enemy hit toward A, out. switch to player serve
      )
      (:`Ball.HeadingTo.Bside`
        (`self.Enemy's Turn to Serve` :!label _label_2)))
    (else
      (`|SwitchGameplayTag` _ball_heading_state ; this happens with the first bounce is in and second bounce is out (swing miss)
        (:`Ball.HeadingTo.Aside`
          (`|SwitchGameplayTag` (`self.TurnToServe`)
            (:`TurnToServe.Player`
              (goto _label_2))
            (:`TurnToServe.Opponent`
              (`self.Increment Opponent Score`)
              (bind _somebody_won_ (`self.Check Win Condition`))
              (if _somebody_won_
                _
                (else
                  (goto _label_2))))))
        (:`Ball.HeadingTo.Bside`
          (`|SwitchGameplayTag` (`self.TurnToServe`)
            (:`TurnToServe.Player`
              (`self.Increment Player Score`)
              (bind _somebody_won__2 (`self.Check Win Condition`))
              (if _somebody_won__2
                _
                (else
                  (goto _label))))
            (:`TurnToServe.Opponent`
              (goto _label)))))))
  (`/Game/BP_Ball_Projectile.Set Ball Heading State` (`self.current ball ref`) (struct :`TagName` "Ball.HeadingTo.Nowhere")))

(fn `send string to paddle`
  (params (msg :type String))
  (bind _returnvalue (`GameplayStatics.GetActorOfClass` "/Game/TestUDP/BP_UDPController.BP_UDPController_C"))
  (bind _asbp_udpcontroller (cast `/Game/TestUDP/BP_UDPController` _returnvalue))
  (`/Game/TestUDP/BP_UDPController.send string to paddle` _asbp_udpcontroller msg))

(fn `UserConstructionScript`)