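; BP_GameBase repeatedly launches short-lived physics balls into the level.
; On BeginPlay, a self-calling SpawnBall event spawns a BP_Ball at SpawnTransform and applies a fixed impulse to its sphere.
; After a short delay it destroys that ball and spawns the next, so the loop runs indefinitely.
; An unconnected fragment for storing the player location never runs, and Tick is empty.
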(event `self.ReceiveBeginPlay`
  (`self.SpawnBall`))

(event `SpawnBall`
  (`KismetSystemLibrary.PrintString` "Spawn Ball")
  (bind _returnvalue (`|SpawnActorFromClass` "/Game/BP_Ball.BP_Ball_C" (`self.Spawn Transform`) "Undefined" "MultiplyWithRoot" null (0.0 0.0 0.0) 1.0 null))
  (`PrimitiveComponent.AddImpulse` (`/Game/BP_Ball.Sphere` _returnvalue) (100.0 0.0 30.0) "None" false)
  (`KismetSystemLibrary.Delay` 3.0)
  (`self.K2_DestroyActor` _returnvalue)
  (`self.SpawnBall`))

(event `self.ReceiveTick`
  (params (DeltaSeconds :type "Float (single-precision)")))

(fn `UserConstructionScript`)