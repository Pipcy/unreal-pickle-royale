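; Game mode for the character select level, previewing the chosen character and paddle on a podium mannequin.
; BeginPlay finds the BP_Chub mannequin, caches BP_GameInstance and applies the current character mesh.
; Separate update events swap the mannequin's skeletal mesh or paddle static mesh and store each choice in the game instance.
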(event `self.ReceiveBeginPlay`
  (bind _returnvalue (`GameplayStatics.GetActorOfClass` "/Game/Player/Chub/BP_Chub.BP_Chub_C"))
  (set `self.mannequin chub` _returnvalue)
  (bind _asbp_game_instance (cast `/Game/UI/BP_GameInstance` (`GameplayStatics.GetGameInstance`)))
  (set `self.game instance ref` _asbp_game_instance)
  (`self.update character mesh`))

(event `update character mesh`
  ; for displayig on the podium
  (`SkeletalMeshComponent.SetSkeletalMeshAsset` (`Character.Mesh` (`self.mannequin chub`)) (`self.choosen character  mesh`))
  ; set game instance
  (set `/Game/UI/BP_GameInstance.Character Selection` (`self.choosen character  mesh`) (`self.game instance ref`)))

(event `update paddle mesh`
  ; for display on the podium
  (`StaticMeshComponent.SetStaticMesh` (`/Game/Player/Chub/BP_Chub.paddle mesh` (`self.mannequin chub`)) (`self.choosen paddle mesh`))
  ; set game instance
  (set `/Game/UI/BP_GameInstance.Paddle Selection` (`self.choosen paddle mesh`) (`self.game instance ref`)))

(fn `UserConstructionScript`)