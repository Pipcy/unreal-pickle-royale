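; PC_UITest is a test player controller that drives the score HUD.
; On BeginPlay it creates WB_HUD, adds it to the viewport, sets Game and UI input mode and pushes the initial scores.
; Debug number keys increment the player or bot score or reset both, each calling UpdateScores on the HUD to refresh the display.
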(event `self.ReceiveBeginPlay`
  (bind _returnvalue (`|CreateWidget` "/Game/UI/WB_HUD.WB_HUD_C"))
  (bind _output_get (set `self.HUDRef` _returnvalue))
  (`UserWidget.AddToViewport` (`self.HUDRef`) 0)
  (`UserWidget.AddToViewport` _output_get 0)
  (`WidgetBlueprintLibrary.SetInputMode_GameAndUIEx` self null)
  (`/Game/UI/WB_HUD.UpdateScores` (`self.HUDRef`) (`self.PlayerScore`) (`self.BotScore`)))

(event `Key|Two`
  (params (Key :type "Key Structure"))
  ; Adding Points Bot + Player
  (:`Pressed`
    (bind _output_get (set `self.BotScore` (+ 1 (`self.BotScore`))))
    (`/Game/UI/WB_HUD.UpdateScores` (`self.HUDRef`) (`self.PlayerScore`) _output_get :!label _label)))

(event `Key|One`
  (params (Key :type "Key Structure"))
  ; Adding Points Bot + Player
  (:`Pressed`
    (set `self.PlayerScore` (+ (`self.PlayerScore`) 1))
    (goto _label)))

(event `Key|Zero`
  (params (Key :type "Key Structure"))
  ; Adding Points Bot + Player
  (:`Pressed`
    (set `self.BotScore` 0)
    (set `self.PlayerScore` 0)
    (`/Game/UI/WB_HUD.UpdateScores` (`self.HUDRef`) 0 0)))

(fn `UserConstructionScript`)